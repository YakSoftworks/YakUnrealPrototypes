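; Player controller for the sprite replication system that lets the player turn the control rotation horizontally.
; On BeginPlay it adds an Enhanced Input mapping context, whose rotate action steps yaw by a fixed amount in the input's direction past a deadzone.
; It caches the possessed BP_PaperCharacter and exposes GetCanUpdateRotation to read that pawn's flag, though the rotate input does not check it.
; Debug prints remain, along with a disconnected timeline rotation.
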(event Custom|LocalSetupInput
  (Input|AddMappingContext (PlayerController|LocalPlayerSubsystems|GetEnhancedInputLocalPlayerSubsystem self) "/Game/Sys_SpriteReplication/Input/IMC_SpriteRepPC.IMC_SpriteRepPC" 0 "(bIgnoreAllPressedKeysUntilRelease=True,bForceImmediately=False,bNotifyUserSettings=False)"))

(event Input|EnhancedActionEvents|EnhancedInputActionIA_TriggerRotate
  (params (ActionValue :type Vector%202D%20Structure) (ElapsedSeconds :type Float%20%28double-precision%29) (TriggeredSeconds :type Float%20%28double-precision%29) (InputAction :type Input%20Action%20Object%20Reference :default "/Game/Sys_SpriteReplication/Input/IA_TriggerRotate.IA_TriggerRotate"))
  (Development|PrintString "Triggered")
  (if (> (Math|Float|Absolute(Float) (.x ActionValue)) 0.25)
    (Pawn|SetControlRotation (Math|Rotator|CombineRotators (Pawn|GetControlRotation :!class /Script/Engine.Controller) (Math|Rotator|MakeRotator 0.0 0.0 (* (Math|Float|Sign(Float) (.x ActionValue)) 0.5))))))

(event EventBeginPlay
  (CallFunction|LocalSetupInput))

(event EventPossess
  (params (PossessedPawn :type Pawn%20Object%20Reference))
  (bind _asbp_paper_character (Utilities|Casting|CastToBP_PaperCharacter PossessedPawn))
  (Variables|Default|SetAs%20BP%20Paper%20Character _asbp_paper_character)
  (Development|PrintString "Got Cast!"))

(event EventUnPossess
  (params (UnpossessedPawn :type Pawn%20Object%20Reference))
  (Variables|Default|SetAs%20BP%20Paper%20Character 0))

(fn ConstructionScript)

(fn GetCanUpdateRotation
  (bind _asbp_paper_character (Utilities|Casting|CastToBP_PaperCharacter (Pawn|GetControlledPawn)))
  (return (Variables|/Game/Sys_SpriteReplication/BP_PaperCharacter.BP_PaperCharacter_C|GetbShouldUpdateRotation _asbp_paper_character)))