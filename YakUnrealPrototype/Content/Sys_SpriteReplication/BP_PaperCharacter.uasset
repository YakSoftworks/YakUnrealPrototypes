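; Paper2D player character that moves relative to camera yaw through Enhanced Input and turns its sprite to face a camera vector.
; Possession adds the input mapping, input records sprint state and last move direction, and BeginPlay hands a sprite data asset to the PaperZD anim instance.
; AdjustSpriteRotation uses 2D dot products to snap the sprite in 90-degree steps.
; The Old Facing graph holds earlier rotation attempts.
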(event Custom|LocalSetupPlayerController
  (params (NewParam :type Player%20Controller%20Object%20Reference))
  (Input|AddMappingContext (PlayerController|LocalPlayerSubsystems|GetEnhancedInputLocalPlayerSubsystem NewParam) "/Game/Sys_SpriteReplication/Input/IMC_SpriteRep.IMC_SpriteRep" 0 "(bIgnoreAllPressedKeysUntilRelease=True,bForceImmediately=False,bNotifyUserSettings=False)"))

(event Custom|UpdateIsSprinting
  (params (Sprint :type Boolean))
  (Variables|Default|SetbIsSprinting Sprint))

(event Custom|UpdateLastInputVector
  (params (InputVector :type Vector))
  (Variables|Default|SetLastInputVector InputVector))

(event Custom|SetShouldUpdateRotation
  (params (NewParam :type Boolean))
  (Variables|Default|SetbShouldUpdateRotation NewParam))

(event Input|EnhancedActionEvents|EnhancedInputActionIA_SpriteRepMove
  (params (ActionValue :type Vector%202D%20Structure) (ElapsedSeconds :type Float%20%28double-precision%29) (TriggeredSeconds :type Float%20%28double-precision%29) (InputAction :type Input%20Action%20Object%20Reference :default "/Game/Sys_SpriteReplication/Input/IA_SpriteRepMove.IA_SpriteRepMove"))
  (bind _returnvalue (Pawn|GetControlRotation :!class /Script/Engine.Pawn))
  (bind (_x _y) (Math|Vector2D|BreakVector2D ActionValue))
  (bind _returnvalue_2 (Math|Rotator|MakeRotator 0.0 0.0 (.yaw _returnvalue)))
  (bind _returnvalue_3 (Math|Vector|GetForwardVector _returnvalue_2))
  (bind _returnvalue_4 (Math|Vector|GetRightVector _returnvalue_2))
  (:Triggered
    (if (Pawn|IsLocallyControlled)
      (Utilities|FlowControl|Sequence
        (:then_0
          (Pawn|Input|AddMovementInput _returnvalue_3 _y false))
        (:then_1
          (Pawn|Input|AddMovementInput _returnvalue_4 _x false))
        (:then_2
          (bind _output_get (Variables|Default|SetLastInputVector (Math|Vector|Normalize (+ (* _returnvalue_3 _y) (* _returnvalue_4 _x)))))
          (CallFunction|UpdateLastInputVector _output_get))))))

(event Input|EnhancedActionEvents|EnhancedInputActionIA_SpriteRepSprint
  (params (ActionValue :type Boolean) (ElapsedSeconds :type Float%20%28double-precision%29) (TriggeredSeconds :type Float%20%28double-precision%29) (InputAction :type Input%20Action%20Object%20Reference :default "/Game/Sys_SpriteReplication/Input/IA_SpriteRepSprint.IA_SpriteRepSprint"))
  (:Started
    (CallFunction|UpdateIsSprinting true))
  (:Completed
    (CallFunction|UpdateIsSprinting false)))

(event Collision|EventActorBeginOverlap
  (params (OtherActor :type Actor%20Object%20Reference)))

(event EventTick
  (params (DeltaSeconds :type Float%20%28single-precision%29)))

(event EventPossessed
  (params (NewController :type Controller%20Object%20Reference))
  (bind _asplayer_controller (Utilities|Casting|CastToPlayerController NewController))
  (CallFunction|LocalSetupPlayerController _asplayer_controller))

(fn ConstructionScript)

(fn AdjustSpriteRotation
  (params (CameraVector :type Vector))
  (bind _sprite (Variables|Default|GetSprite))
  (bind _sprite_2 (Variables|Default|GetSprite))
  (bind _returnvalue (Math|Vector|GetForwardVector _sprite))
  (bind _returnvalue_2 (Math|Vector|GetRightVector _sprite_2))
  (bind _output_get (LocalVariables|SetForwardDot (Math|Vector2D|DotProduct(2D) (Math|Vector2D|MakeVector2D (.x CameraVector) (.y CameraVector)) (Math|Vector2D|MakeVector2D (.x _returnvalue) (.y _returnvalue)))))
  (if (<= _output_get (* (Math|Trig|Cos(Degrees) 45.0) -1.0)) ; Check if at acceptable angle
    (return) ; Within 45deg from ortho angle
    (elif (>= (LocalVariables|GetForwardDot) (Math|Trig|Cos(Degrees) 45.0)) ; Backwards Case
      ;[0.15 0.15 0.15 0.5] Rotate 180
      (Transformation|AddRelativeRotation (Variables|Default|GetSprite) "0.000000,180.000000,0.000000" false false)
      (return)
      (else
        (bind _output_get_2 (LocalVariables|SetRightDot (Math|Vector2D|DotProduct(2D) (Math|Vector2D|MakeVector2D (.x _returnvalue_2) (.y _returnvalue_2)) (Math|Vector2D|MakeVector2D (.x CameraVector) (.y CameraVector)))))
        (if (> (Math|Float|Sign(Float) _output_get_2) 0.0)
          ;[0.15 0.15 0.15 0.5] Rotate 90 CW
          (Transformation|AddRelativeRotation (Variables|Default|GetSprite) "0.000000,90.000000,0.000000" false false)
          (return)
          (else
            ;[0.15 0.15 0.15 0.5] Rotate 90 CCW
            (Transformation|AddRelativeRotation (Variables|Default|GetSprite) "0.000000,-90.000000,0.000000" false false)
            (return)))))))

(fn GetXYOrthoVectorfromVector
  (params (QueryVector :type Vector))
  (bind _returnvalue (Math|Vector2D|MakeVector2D 1.0 0.0))
  (bind _returnvalue_2 (Math|Trig|Cos(Degrees) 45.0))
  (bind _returnvalue_3 (Math|Vector|Normalize (Math|Vector|MakeVector (.x QueryVector) (.y QueryVector) 0.0)))
  (bind _returnvalue_4 (Math|Conversions|ToVector2D(Vector) _returnvalue_3))
  (bind _returnvalue_5 (Math|Vector2D|DotProduct(2D) _returnvalue _returnvalue_4))
  (if (>= _returnvalue_5 _returnvalue_2) ; Check if at acceptable angle
    (return "(X=1.000000,Y=0.000000)") ; Within 45deg from ortho angle
    (elif (<= _returnvalue_5 (* _returnvalue_2 -1.0)) ; Backwards Case
      (return "(X=-1.000000,Y=0.000000)")
      (elif (> (Math|Vector2D|DotProduct(2D) (Math|Vector2D|MakeVector2D 0.0 1.0) (Math|Conversions|ToVector2D(Vector) QueryVector)) 0.0) ; Check if at acceptable angle
        (return "(X=0.000000,Y=1.000000)") ; Within 45deg from ortho angle
        (else
          (return "(X=0.000000,Y=-1.000000)"))))))

(event Custom|SetRelativeLocalRotation
  (params (LocalCameraDirection :type Vector))
  (bind _sprite (Variables|Default|GetSprite))
  (if (Math|Float|NearlyEqual(Float) (.yaw (Variables|/Script/Engine.SceneComponent|GetRelativeRotation (Variables|Default|GetSprite))) 0.0 0.001)
    (Transformation|SetRelativeRotation _sprite "0.000000,90.000000,0.000000" false false)
    (Development|PrintString (Utilities|String|Append "Setting to 90: " (Utilities|GetDisplayName self)) false false)
    (else
      (Transformation|SetRelativeRotation _sprite "0, 0, 0" false false)
      (Development|PrintString (Utilities|String|Append "Setting to 0 : " (Utilities|GetDisplayName self)) false false)))
  (if (> (Math|Vector|DotProduct LocalCameraDirection (Math|Vector|GetForwardVector (Variables|Default|GetSprite))) 0.0)
    (Transformation|AddWorldRotation (Variables|Default|GetSprite) "0.000000,180.000000,0.000000" false false)))

(event Custom|MakeSpriteFaceCamera
  (params (CameraVector :type Vector))
  (bind _sprite (Variables|Default|GetSprite))
  (bind _returnvalue (Math|Vector|GetForwardVector _sprite))
  (bind _returnvalue_2 (Math|Vector|DotProduct CameraVector _returnvalue))
  (bind _returnvalue_3 (Math|Vector|CrossProduct CameraVector _returnvalue))
  (bind _returnvalue_4 (Math|Vector|VectorLength _returnvalue_3))
  (bind _returnvalue_5 (Class|KismetMathLibrary|DegAsin _returnvalue_4))
  (bind _returnvalue_6 (Math|Float|Sign(Float) _returnvalue_5))
  ;[1 1 1] First Check Dot Product - Cos
  (if (Math|Float|NearlyEqual(Float) _returnvalue_2 -1.0 0.01) ; Check if -1, if so, we can stop
    (Development|PrintString "No need to rotate" false false)
    (elif (Math|Float|NearlyEqual(Float) _returnvalue_2 1.0 0.01) ; Check if 1 - If so, rotate by 180
      (Transformation|AddRelativeRotation (Variables|Default|GetSprite) "0.000000,180.000000,0.000000" false false)
      (Development|PrintString "Rotation Case 1")
      (else
        ;[1 1 1] If still invalid, check the cross product - Sin
        (if (Math|Float|NearlyEqual(Float) _returnvalue_6 1.0 0.01) ; If need to rotate CW
          (Transformation|AddRelativeRotation (Variables|Default|GetSprite) "0.000000,-90.000000,0.000000" false false)
          (Development|PrintString "Rotation Case 2")
          (elif (Math|Float|NearlyEqual(Float) _returnvalue_6 -1.0 0.01)
            (Transformation|AddRelativeRotation (Variables|Default|GetSprite) "0.000000,90.000000,0.000000" false false)
            (Development|PrintString "Rotation Case 3")
            (else
              (Development|PrintString "Invalid Rotation Case" true true "(R=1.000000,G=0.000000,B=0.048144,A=1.000000)"))))))))

(event EventBeginPlay
  (bind _aszdabp_celes (Utilities|Casting|CastToZDABP_Celes (Variables|/Script/PaperZD.PaperZDAnimationComponent|GetAnimInstance (Variables|Default|GetPaperZDAnimation))))
  (Variables|/Game/Sys_SpriteReplication/ZDABP_Celes.ZDABP_Celes_C|SetAnimDataAsset _aszdabp_celes (Variables|Default|GetSpriteDataAsset)))