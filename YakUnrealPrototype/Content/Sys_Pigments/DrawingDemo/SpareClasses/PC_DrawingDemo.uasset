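; Player controller for a pigment drawing demo that creates the drawing UI, shows the cursor and clears the paint render targets on start.
; Each left click stamps a polygon dot at the cursor into active scattering and absorption targets, using the UI's current S and K values.
; OnDry draws composite materials into dry reflectance and transmittance targets, modeling paint as optical layers rather than plain color.
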(event Custom|OnAddDot
  (bind _uiref (Variables|Default|GetUIRef))
  (bind _uiref_2 (Variables|Default|GetUIRef))
  (bind _radius (Variables|Default|GetRadius))
  (bind _radius_2 (Variables|Default|GetRadius))
  (bind _currentabsorbtion_k_ (Variables|/Game/Sys_Pigments/DrawingDemo/WBP_DrawingUI.WBP_DrawingUI_C|GetCurrentAbsorbtion%28K%29 _uiref))
  (bind _currentscattering_s_ (Variables|/Game/Sys_Pigments/DrawingDemo/WBP_DrawingUI.WBP_DrawingUI_C|GetCurrentScattering%28S%29 _uiref_2))
  (Utilities|FlowControl|Sequence
    (:then_0
      (bind (_canvas _size _context) (Rendering|BeginDrawCanvastoRenderTarget (Variables|Default|GetRTarget_Active_Scatter)))
      (bind _returnvalue (Class|WidgetLayoutLibrary|GetMousePositiononViewport))
      (Class|Canvas|DrawPolygon _canvas 0 _returnvalue (Math|Vector2D|MakeVector2D _radius_2 _radius_2) 12 (Utilities|Struct|MakeLinearColor (.x _currentscattering_s_) (.y _currentscattering_s_) (.z _currentscattering_s_) 1.0))
      (Rendering|EndDrawCanvastoRenderTarget _context))
    (:then_1
      (bind (_canvas_2 _size_2 _context_2) (Rendering|BeginDrawCanvastoRenderTarget (Variables|Default|GetRTarget_Active_Absorb)))
      (bind _returnvalue_2 (Class|WidgetLayoutLibrary|GetMousePositiononViewport))
      (Class|Canvas|DrawPolygon _canvas_2 0 _returnvalue_2 (Math|Vector2D|MakeVector2D _radius _radius) 12 (Utilities|Struct|MakeLinearColor (.x _currentabsorbtion_k_) (.y _currentabsorbtion_k_) (.z _currentabsorbtion_k_) 1.0))
      (Rendering|EndDrawCanvastoRenderTarget _context_2))))

(event Custom|OnDry
  (Utilities|FlowControl|Sequence
    (:then_0
      (bind (_canvas _size _context) (Rendering|BeginDrawCanvastoRenderTarget "/Game/Sys_Pigments/DrawingDemo/RenderTargest/Try2/RT_Dry_Reflectance.RT_Dry_Reflectance"))
      (Canvas|DrawMaterial :self _canvas :RenderMaterial "/Game/Sys_Pigments/DrawingDemo/RenderTargest/Try2/M_CompositveReflectance.M_CompositveReflectance" :ScreenSize "(X=1280.000000,Y=720.000000)" :CoordinateSize "(X=1.000000,Y=1.000000)" :PivotPoint "(X=0.000000,Y=0.000000)")
      (Rendering|EndDrawCanvastoRenderTarget _context))
    (:then_1
      (bind (_canvas_2 _size_2 _context_2) (Rendering|BeginDrawCanvastoRenderTarget "/Game/Sys_Pigments/DrawingDemo/RenderTargest/Try2/RT_Dry_Transmittance.RT_Dry_Transmittance"))
      (Canvas|DrawMaterial :self _canvas_2 :RenderMaterial "/Game/Sys_Pigments/DrawingDemo/RenderTargest/Try2/M_CompositeTransmittance.M_CompositeTransmittance" :ScreenSize "(X=1280.000000,Y=720.000000)" :CoordinateSize "(X=1.000000,Y=1.000000)" :PivotPoint "(X=0.000000,Y=0.000000)")
      (Rendering|EndDrawCanvastoRenderTarget _context_2))))

(event EventBeginPlay
  (bind _returnvalue (UserInterface|CreateWidget "/Game/Sys_Pigments/DrawingDemo/WBP_DrawingUI.WBP_DrawingUI_C" self))
  (bind _output_get (Variables|Default|SetUIRef _returnvalue))
  (UserInterface|Viewport|AddtoViewport _output_get 0)
  (Class|GameplayStatics|SetViewportMouseCaptureMode "NoCapture")
  (Variables|Default|SetbShowMouseCursor true)
  ;[0.15 0.15 0.15 0.5] Reset Textures On Start
  (Rendering|ClearRenderTarget2D (Variables|Default|GetRTarget_Active_Scatter) "(R=1.000000,G=1.000000,B=1.000000,A=0.000000)")
  (Rendering|ClearRenderTarget2D (Variables|Default|GetRTarget_Active_Absorb) "(R=1.000000,G=1.000000,B=1.000000,A=0.000000)")
  (Rendering|ClearRenderTarget2D (Variables|Default|GetRTarget_Dry_Reflectance) "(R=1.000000,G=1.000000,B=1.000000,A=0.000000)")
  (Rendering|ClearRenderTarget2D (Variables|Default|GetRTarget_Dry_Transmittance) "(R=1.000000,G=1.000000,B=1.000000,A=0.000000)"))

(event EventTick
  (params (DeltaSeconds :type Float%20%28single-precision%29)))

(event Input|MouseEvents|DebugKeyLeftMouseButton
  (params (Key :type Key%20Structure :default "None") (ActionValue :type Input%20Action%20Value%20Structure))
  (:Pressed
    (CallFunction|OnAddDot)))

(fn ConstructionScript)

(fn IsMouseOverImage)